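; Game mode for a maze level that runs a countdown and shows the You_Lose widget when time runs out.
; A looping one-second timer decrements the Timer variable, creating and adding the widget on every tick at or below zero.
; At BeginPlay it also binds to the third-person character's DPLightColor and DPLightRed dispatchers, either of which stops the countdown.
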(event Custom|Time
  (bind _result (Math|Integer|DecrementInt (Variables|Default|GetTimer))
    (:%20%20
      (Variables|Default|SetTimer _result)
      (if (<= (Variables|Default|GetTimer) 0)
        (bind _returnvalue (UserInterface|CreateWidget "/Game/LabWork_Maze/You_Lose.You_Lose_C"))
        (UserInterface|Viewport|AddtoViewport _returnvalue 0)))))

(event Custom|Y
  (Utilities|Time|ClearTimerbyFunctionName 0 "Time"))

(event Custom|Light_Red
  (Utilities|Time|ClearTimerbyFunctionName 0 "Time"))

(event EventBeginPlay
  (Utilities|Time|SetTimerbyFunctionName 0 "Time" 1.0 true)
  (bind _asbp_third_person_character (Utilities|Casting|CastToBP_ThirdPersonCharacter (Game|GetPlayerCharacter 0)))
  (bind _output_get (Variables|Default|SetAs%20BP%20Third%20Person%20Character _asbp_third_person_character))
  (EventDispatchers|BindEventtoDPLightColor _output_get (delegate Custom|Y))
  (EventDispatchers|BindEventtoDPLightRed _output_get (delegate Custom|Light_Red)))

(fn ConstructionScript)