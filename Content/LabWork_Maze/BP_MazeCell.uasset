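; BP_MazeCell is a modular maze cell actor with configurable walls, floor, ceiling and light.
; Its construction script scales the floor from GridSize and adds cube meshes for each enabled wall and ceiling, using SizeToCubeScale for dimensions.
; A ceiling with positive LightIntensity also gets a colored point light.
; On BeginPlay it binds to the third-person character's DPLightColor and DPLightRed dispatchers, which turn that light green or red.
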(event Custom|Light
  (Rendering|Components|Light|SetLightColor (Variables|Default|GetNewVar) "(R=0.000000,G=1.000000,B=0.017720,A=1.000000)" true))

(event Custom|Red_Light
  (Rendering|Components|Light|SetLightColor (Variables|Default|GetNewVar) "(R=1.000000,G=0.000000,B=0.000000,A=1.000000)" true))

(event EventBeginPlay
  (bind _asbp_third_person_character (Utilities|Casting|CastToBP_ThirdPersonCharacter (Game|GetPlayerCharacter 0)))
  (bind _output_get (Variables|Default|SetAs%20BP%20Third%20Person%20Character _asbp_third_person_character))
  (EventDispatchers|BindEventtoDPLightColor _output_get (delegate Custom|Light))
  (EventDispatchers|BindEventtoDPLightRed _output_get (delegate Custom|Red_Light)))

(event Collision|EventActorBeginOverlap
  (params (OtherActor :type Actor%20Object%20Reference)))

(event EventTick
  (params (DeltaSeconds :type Float%20%28single-precision%29)))

(fn ConstructionScript
  (bind _grid_size (Variables|Default|GetGrid_Size))
  (LocalVariables|SetWall_Thicness (* _grid_size 0.1))
  (LocalVariables|SetWall_Lenght _grid_size)
  (Transformation|SetRelativeScale3D (Variables|Default|GetFloor) (Utilities|SizetoCubeScale (Math|Vector|MakeVector (LocalVariables|GetWall_Lenght) (LocalVariables|GetWall_Lenght) (LocalVariables|GetWall_Thicness))))
  (if (Variables|Default|GetWest_Wall)
    (AddComponent|AddStaticMeshComponent false (Math|Transform|MakeTransform "0, 0, 0" "0, 0, 0" (Utilities|SizetoCubeScale (Math|Vector|MakeVector (LocalVariables|GetWall_Lenght) (LocalVariables|GetWall_Thicness) (Variables|Default|GetWall_Height))))))
  (if (Variables|Default|GetSouth_Wall)
    (AddComponent|AddStaticMeshComponent false (Math|Transform|MakeTransform "0, 0, 0" "0, 0, 0" (Utilities|SizetoCubeScale (Math|Vector|MakeVector (LocalVariables|GetWall_Thicness) (LocalVariables|GetWall_Lenght) (Variables|Default|GetWall_Height))))))
  (if (Variables|Default|GetNorth_Wall)
    (AddComponent|AddStaticMeshComponent false (Math|Transform|MakeTransform (Math|Vector|MakeVector (- (LocalVariables|GetWall_Lenght) (LocalVariables|GetWall_Thicness)) 0.0 0.0) "0, 0, 0" (Utilities|SizetoCubeScale (Math|Vector|MakeVector (LocalVariables|GetWall_Thicness) (LocalVariables|GetWall_Lenght) (Variables|Default|GetWall_Height))))))
  (if (Variables|Default|GetEast_Wall)
    (AddComponent|AddStaticMeshComponent false (Math|Transform|MakeTransform (Math|Vector|MakeVector 0.0 (- (LocalVariables|GetWall_Lenght) (LocalVariables|GetWall_Thicness)) 0.0) "0, 0, 0" (Utilities|SizetoCubeScale (Math|Vector|MakeVector (LocalVariables|GetWall_Lenght) (LocalVariables|GetWall_Thicness) (Variables|Default|GetWall_Height))))))
  (if (Variables|Default|GetCieling)
    (AddComponent|AddStaticMeshComponent false (Math|Transform|MakeTransform (Math|Vector|MakeVector 0.0 0.0 (- (LocalVariables|GetWall_Lenght) (LocalVariables|GetWall_Thicness))) "0, 0, 0" (Utilities|SizetoCubeScale (Math|Vector|MakeVector (LocalVariables|GetWall_Lenght) (LocalVariables|GetWall_Lenght) (LocalVariables|GetWall_Thicness)))))
    (if (> (Variables|Default|GetLight_Intensity) 0.0)
      (bind _returnvalue (AddComponent|AddPointLightComponent false (Math|Transform|MakeTransform (Math|Vector|MakeVector (* (LocalVariables|GetWall_Lenght) 0.5) (* (LocalVariables|GetWall_Lenght) 0.5) (* (Variables|Default|GetWall_Height) 0.75)) "0, 0, 0" "1.000000,1.000000,1.000000")))
      (Variables|Default|SetNewVar _returnvalue)
      (Rendering|Components|Light|SetLightColor _returnvalue (Variables|Default|GetLight_Color) true)
      (Rendering|Components|Light|SetIntensity _returnvalue (Variables|Default|GetLight_Intensity)))))